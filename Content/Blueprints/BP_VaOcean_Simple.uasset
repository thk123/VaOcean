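; BP_VaOcean_Simple is an ocean surface actor whose material is driven by the level's VaOcean state actor.
; On BeginPlay it finds the simple state actor, puts a dynamic M_OceanSimple instance on its mesh and copies in the wave, panner and water height settings.
; Tick feeds game time into the material's wave height panner, so the material's wave animation follows the game clock.
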(event `self.ReceiveTick`
  (params (DeltaSeconds :type "Float (single-precision)"))
  (`MaterialInstanceDynamic.SetScalarParameterValue` (`self.OceanMaterial`) "WaveHeightPannerTime" (`KismetSystemLibrary.GetGameTimeInSeconds`)))

(event `self.ReceiveBeginPlay`
  (bind _oceanmaterial (`self.OceanMaterial`))
  (bind _outactors (`GameplayStatics.GetAllActorsOfClass` "/Script/VaOceanPlugin.VaOceanStateActor"))
  (for _array_element _outactors
    (bind _asvaoceanstateactorsimple (cast `VaOceanStateActorSimple` _array_element))
    ;[1 1 1] Ocean material
    (bind _returnvalue (`KismetMaterialLibrary.CreateDynamicMaterialInstance` "/VaOceanPlugin/Materials/M_OceanSimple.M_OceanSimple"))
    (set `self.OceanMaterial` _returnvalue)
    (`PrimitiveComponent.SetMaterial` (`self.StaticMesh1`) 0 (`self.OceanMaterial`))
    ;[1 1 1] Ocean instance setup
    (`MaterialInstanceDynamic.SetScalarParameterValue` _oceanmaterial "WorldPositionDivider" (`VaOceanStateActorSimple.GetWorldPositionDivider` _asvaoceanstateactorsimple))
    (`MaterialInstanceDynamic.SetScalarParameterValue` _oceanmaterial "WaveUVDivider" (`VaOceanStateActorSimple.GetWaveUVDivider` _asvaoceanstateactorsimple))
    (`MaterialInstanceDynamic.SetScalarParameterValue` _oceanmaterial "WaveHeightPannerX" (`VaOceanStateActorSimple.GetWaveHeightPannerX` _asvaoceanstateactorsimple))
    (`MaterialInstanceDynamic.SetScalarParameterValue` _oceanmaterial "WaveHeightPannerY" (`VaOceanStateActorSimple.GetWaveHeightPannerY` _asvaoceanstateactorsimple))
    (`MaterialInstanceDynamic.SetScalarParameterValue` _oceanmaterial "WaveHeight" (`VaOceanStateActorSimple.GetWaveHeight` _asvaoceanstateactorsimple))
    (`MaterialInstanceDynamic.SetScalarParameterValue` _oceanmaterial "WaterHeight" (`VaOceanStateActorSimple.GetWaterHeight` _asvaoceanstateactorsimple))))

(fn `UserConstructionScript`)